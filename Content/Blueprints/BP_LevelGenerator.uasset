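; Procedural level generator that, on BeginPlay, spawns a random start room, a chain of main rooms, an end room, then branch rooms.
; BuildRoom attaches random room classes to a parent's random door, retrying a few times before destroying that door.
; The main path backtracks by deleting its last room when no doors remain, resetting the start room's doors if emptied.
; Branches then grow from each main room until capped or blocked.
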(event EventBeginPlay
  (CallFunction|BuildRooms))

(event Collision|EventActorBeginOverlap
  (params (OtherActor :type Actor%20Object%20Reference)))

(event EventTick
  (params (DeltaSeconds :type Float%20%28single-precision%29)))

(fn ConstructionScript)

(fn BuildRooms
  (bind _mainrooms (LocalVariables|GetMainRooms))
  (bind _mainrooms_2 (LocalVariables|GetMainRooms))
  (bind _mainrooms_3 (LocalVariables|GetMainRooms))
  (bind _mainrooms_4 (LocalVariables|GetMainRooms))
  (bind _mainrooms_5 (LocalVariables|GetMainRooms))
  (bind _returnvalue (Utilities|Array|LastIndex _mainrooms_3))
  (bind _returnvalue_2 (Utilities|Array|LastIndex _mainrooms_5))
  (bind _output (Utilities|Array|Get(acopy) _mainrooms_5 _returnvalue_2))
  (bind _output_2 (Utilities|Array|Get(acopy) _mainrooms_3 _returnvalue))
  (bind _spawnedroom (CallFunction|BuildRoom (Variables|Default|GetStartRooms)))
  (LocalVariables|SetStartRoom _spawnedroom)
  (while (not (LocalVariables|GetIsFinished))
    (if (< (Utilities|Array|Length (LocalVariables|GetMainRooms)) (Variables|Default|GetMainRoomCount))
      (if (> (Utilities|Array|Length (LocalVariables|GetMainRooms)) 0)
        (bind _spawnedroom_2 (CallFunction|BuildRoom (Variables|Default|GetRooms) _output))
        (Utilities|IsValid _spawnedroom_2
          (:Is%20Valid
            (Utilities|Array|Add (LocalVariables|GetMainRooms) _spawnedroom_2))
          (:Is%20Not%20Valid
            (bind _door (Default|GetRandomDoor _output))
            (Utilities|IsValid _door
              (:Is%20Not%20Valid
                (Development|PrintString (Utilities|String|Append "Deleted - " (Utilities|GetDisplayName _output)))
                (Actor|DestroyActor _output)
                (Utilities|Array|RemoveIndex _mainrooms_4 (Utilities|Array|LastIndex _mainrooms_4))))))
        (else
          (Default|ResetDoors (LocalVariables|GetStartRoom)) ; Reset Doors to Available, for the Start Room, as needed when the second room is Destroyed due to a branch not being valid
          (bind _spawnedroom_3 (CallFunction|BuildRoom (Variables|Default|GetRooms) (LocalVariables|GetStartRoom)))
          (Utilities|IsValid _spawnedroom_3
            (:Is%20Valid
              (Utilities|Array|Add (LocalVariables|GetMainRooms) _spawnedroom_3)))))
      (else
        (bind _spawnedroom_4 (CallFunction|BuildRoom (Variables|Default|GetEndRooms) _output_2))
        (Utilities|IsValid _spawnedroom_4
          (:Is%20Valid
            (LocalVariables|SetIsFinished true))
          (:Is%20Not%20Valid
            (Default|GetRandomDoor _output_2)
            (Utilities|IsValid 0
              (:Is%20Not%20Valid
                (Development|PrintString (Utilities|String|Append "Deleted 2 - " (Utilities|GetDisplayName _output_2)))
                (Actor|DestroyActor _output_2)
                (Utilities|Array|RemoveIndex _mainrooms_2 (Utilities|Array|LastIndex _mainrooms_2)))))))))
  (Development|PrintString "Building Branch Rooms")
  (for _array_element _mainrooms
    (CallFunction|BuildBranchRooms _array_element (Variables|Default|GetMaxBranchRoomCount)))
  (Development|PrintString (Utilities|String|ToString(Integer) (Utilities|Array|Length _mainrooms))))

(fn BuildRoom
  (params (Rooms :type Array%20of%20BP%20Room%20Class%20References) (ParentRoom :type BP%20Room%20Object%20Reference))
  (Utilities|IsValid ParentRoom
    (:Is%20Valid
      (bind _door (Default|GetRandomDoor ParentRoom))
      (Utilities|IsValid _door
        (:Is%20Valid
          (for _index (range 0 4)
            (bind _returnvalue (Game|SpawnActorfromClass (.OutItem (Utilities|Array|Random Rooms)) (Math|Transform|MakeTransform "0, 0, 0" "0, 0, 0" "1,1,1") "Undefined" 0 _door 0)) ; Could do an Overlap check before spawning to see if there would be space for the smallest BP_Room
            (Utilities|IsValid _returnvalue
              (:Is%20Valid
                (Variables|/Game/Blueprints/BP_Door.BP_Door_C|SetIsAvailable _door false)
                (Development|PrintString (Utilities|String|Append (Utilities|GetDisplayName ParentRoom) " -> " (Utilities|GetDisplayName _returnvalue)))
                (return _returnvalue))))
          (Default|DestroyDoor ParentRoom _door)
          (return 0))
        (:Is%20Not%20Valid
          (return 0))))
    (:Is%20Not%20Valid
      (bind _returnvalue_2 (Game|SpawnActorfromClass (.OutItem (Utilities|Array|Random Rooms)) (Math|Transform|MakeTransform "0, 0, 0" (Math|Rotator|MakeRotator 0.0 0.0 (Math|Random|RandomFloatinRange 0.0 3.6e+02)) "1,1,1") "Undefined" 0 0 0))
      (return _returnvalue_2))))

(fn BuildBranchRooms
  (params (ParentRoom :type BP%20Room%20Object%20Reference) (MaxRoomCount :type Integer))
  (bind _branchrooms (LocalVariables|GetBranchRooms))
  (while (< (Utilities|Array|Length (LocalVariables|GetBranchRooms)) MaxRoomCount)
    (if (> (Utilities|Array|Length (LocalVariables|GetBranchRooms)) 0)
      (bind _spawnedroom (CallFunction|BuildRoom (Variables|Default|GetRooms) (Utilities|Array|Get(acopy) _branchrooms (Utilities|Array|LastIndex _branchrooms))))
      (Utilities|IsValid _spawnedroom
        (:Is%20Valid
          (Utilities|Array|Add (LocalVariables|GetBranchRooms) _spawnedroom))
        (:Is%20Not%20Valid
          (return)))
      (else
        (bind _spawnedroom_2 (CallFunction|BuildRoom (Variables|Default|GetRooms) ParentRoom))
        (Utilities|IsValid _spawnedroom_2
          (:Is%20Valid
            (Utilities|Array|Add (LocalVariables|GetBranchRooms) _spawnedroom_2))
          (:Is%20Not%20Valid
            (return)))))))